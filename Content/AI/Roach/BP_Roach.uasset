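; BP_Roach is a 2D flipbook roach character that starts young, can switch to one of three adult looks, and dies after a fixed lifespan.
; Tick picks idle or moving animation from velocity and flips the sprite's rotation by the sign of Y velocity.
; Eat and egg-laying events pause that update while they play; eating always uses the young set.
; Death, triggered by the BeginPlay timer, plays once before destroying the actor.
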(event Custom|LifeContDown
  ;[0.5842 1 0] Comment
  (CallFunction|DieDieDie))

(event Custom|SwitchRoachType
  (params (Selection :type Integer))
  (switch int Selection
    (:Default
      (Variables|Default|SetSelectedPF (Variables|Default|GetAnim_Adult1) :!label _label))
    (:0
      (goto _label))
    (:1
      (Variables|Default|SetSelectedPF (Variables|Default|GetAnim_Adult2)))
    (:2
      (Variables|Default|SetSelectedPF (Variables|Default|GetAnim_Adult3)))))

(event Custom|PLay%20eat%20animation
  (Variables|Default|SetCanMove false)
  (Sprite|SetFlipbook (Variables|Default|GetPaperFlipbook) (Utilities|Array|Get(acopy) (Variables|Default|GetAnim_Young) 4))
  (Utilities|FlowControl|Delay 3.0)
  (Variables|Default|SetCanMove true))

(event Custom|Play%20Lay%20Egg%20Animation
  (Variables|Default|SetCanMove false)
  (Sprite|SetFlipbook (Variables|Default|GetPaperFlipbook) (Utilities|Array|Get(acopy) (Variables|Default|GetSelectedPF) 2))
  (Utilities|FlowControl|Delay 3.0)
  (Variables|Default|SetCanMove true))

(event Custom|DieDieDie
  (bind _paperflipbook (Variables|Default|GetPaperFlipbook))
  (Variables|Default|SetCanMove false)
  (Sprite|SetFlipbook _paperflipbook (Utilities|Array|Get(acopy) (Variables|Default|GetSelectedPF) 3))
  (Components|Timeline|SetLooping _paperflipbook false)
  (Components|Timeline|PlayfromStart _paperflipbook)
  (Utilities|FlowControl|Delay 1.0)
  (Actor|DestroyActor))

(event EventBeginPlay
  ;[0.5842 1 0] Comment
  (Utilities|Time|SetTimerbyEvent (delegate Custom|LifeContDown) 3e+01)
  (Variables|Default|SetCanMove true))

(event EventTick
  (params (DeltaSeconds :type Float%20%28single-precision%29))
  (bind _paperflipbook (Variables|Default|GetPaperFlipbook))
  (bind _paperflipbook_2 (Variables|Default|GetPaperFlipbook))
  (bind _selectedpf (Variables|Default|GetSelectedPF))
  (if (Variables|Default|GetCanMove)
    (Utilities|FlowControl|Sequence
      (:then_1
        (if (== (Math|Vector|VectorLength (Transformation|GetVelocity)) 0.0)
          (Sprite|SetFlipbook _paperflipbook_2 (Utilities|Array|Get(acopy) _selectedpf))
          (else
            (Sprite|SetFlipbook _paperflipbook_2 (Utilities|Array|Get(acopy) _selectedpf 1)))))
      (:then_2
        (Math|Float|CompareFloat (.y (Transformation|GetVelocity)) 0.0
          (:>
            (Transformation|SetRelativeRotation _paperflipbook "0.000000,90.000000,-90.000000" false false))
          (:<
            (Transformation|SetRelativeRotation _paperflipbook "0.000000,-90.000000,90.000000" false false)))))))

(fn ConstructionScript
  (Variables|Default|SetSelectedPF (Variables|Default|GetAnim_Young)))
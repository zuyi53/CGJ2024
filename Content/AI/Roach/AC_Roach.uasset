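; AI controller for the roach that starts its blackboard and behavior tree when play begins.
; On BeginPlay it sets up BB_roach, writes its LifeTime variable and a random Type of 0 or 1 as integer keys, then runs BT_roach.
; The controller holds no further logic beyond seeding these values for the tree.
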(event EventBeginPlay
  (bind _blackboardcomponent (Class|AIController|UseBlackboard "/Game/AI/Roach/BB_roach.BB_roach"))
  (Variables|Default|SetBlackboard%20Component _blackboardcomponent)
  (Class|BlackboardComponent|SetValueasInt (Variables|Default|GetBlackboard%20Component) (Utilities|String|StringToName "LifeTime") (Variables|Default|GetLifeTime))
  (Class|BlackboardComponent|SetValueasInt (Variables|Default|GetBlackboard%20Component) (Utilities|String|StringToName "Type") (Math|Random|RandomInteger 2))
  (AI|RunBehaviorTree "/Game/AI/Roach/BT_roach.BT_roach"))

(fn ConstructionScript)
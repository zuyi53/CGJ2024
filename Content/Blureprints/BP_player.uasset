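; BP_player is a player creature Blueprint that eats food and lays eggs.
; Capsule overlap with a BP_food stores it and sets CanEat; Eatfood destroys that food and sets CanLayEgg, letting TrytoLayEgg spawn a BP_egg at the actor's X/Y.
; The construction script shows either the PlaneH or Plane component based on IsAdult.
; On destruction, it tells BP_Controller to rebind the camera through BindCamera.
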(event OnComponentBeginOverlap(CapsuleComponent)
  (params (OverlappedComponent :type Primitive%20Component%20Object%20Reference) (OtherActor :type Actor%20Object%20Reference) (OtherComp :type Primitive%20Component%20Object%20Reference) (OtherBodyIndex :type Integer) (bFromSweep :type Boolean) (SweepResult :type Hit%20Result%20Structure%20%28by%20ref%29))
  (bind (_asbp_food _bsuccess) (Utilities|Casting|CastToBP_food OtherActor))
  (if _bsuccess
    (Variables|Default|Setfood _asbp_food)
    (Variables|Default|SetCanEat true)
    (Development|PrintString "you can eat")))

(event Custom|Try%20to%20Lay%20Egg
  (bind _returnvalue (Transformation|GetActorLocation))
  ;[1 1 1] Lay egg
  (if (Variables|Default|GetCanLayEgg)
    (Game|SpawnActorfromClass "/Game/Blureprints/BP_egg.BP_egg_C" (Math|Transform|MakeTransform (Math|Vector|MakeVector (.x _returnvalue) (.y _returnvalue) 0.0) "0, 0, 0" "1.000000,1.000000,1.000000") "Undefined" "MultiplyWithRoot" 0 0)
    (Development|PrintString "you have lay an egg")))

(event Custom|Eat%20food
  (bind _food (Variables|Default|Getfood))
  ;[1 1 1] Eat food
  (Utilities|IsValid _food
    (:Is%20Valid
      (Actor|DestroyActor _food)
      (Development|PrintString "you have eat a food")
      (Variables|Default|SetCanLayEgg true)
      (Variables|Default|SetCanEat false))))

(event EventDestroyed
  (Default|BindCamera (.AsBP%20Controller (Utilities|Casting|CastToBP_Controller (Game|GetPlayerController 0)))))

(fn ConstructionScript
  (if (Variables|Default|GetIsAdult)
    (Rendering|SetVisibility (Variables|Default|GetPlaneH) true false)
    (Rendering|SetVisibility (Variables|Default|GetPlane) false false)
    (else
      (Rendering|SetVisibility (Variables|Default|GetPlane) true false)
      (Rendering|SetVisibility (Variables|Default|GetPlaneH) false false))))
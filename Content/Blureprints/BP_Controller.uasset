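; Player controller that drives BP_player's movement and an ability for eating food and laying eggs.
; BeginPlay adds the Enhanced Input context, caches the pawn and switches the view to the first BP_Camera in the level.
; Move input maps to world axes; the ability destroys edible food, enabling egg laying, then spawns BP_egg at the player whenever allowed.
; Cursor/touch trace, follow and click-to-move helpers are defined but not called in this graph.
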(event Input|EnhancedActionEvents|EnhancedInputActionIA_abiliy1
  (params (ActionValue :type Boolean) (ElapsedSeconds :type Float%20%28double-precision%29) (TriggeredSeconds :type Float%20%28double-precision%29) (InputAction :type Input%20Action%20Object%20Reference :default "/Game/Input/Actions/IA_abiliy1.IA_abiliy1"))
  (bind _bp_player (Variables|Default|GetBp%20player))
  (bind _food (Variables|/Game/Blureprints/BP_player.BP_player_C|Getfood _bp_player))
  (:Started
    (Utilities|FlowControl|Sequence
      (:then_0
        (if (Variables|/Game/Blureprints/BP_player.BP_player_C|GetCanEat _bp_player)
          (Utilities|IsValid _food
            (:Is%20Valid
              (Actor|DestroyActor _food)
              (Development|PrintString "you have eat a food")
              (Variables|/Game/Blureprints/BP_player.BP_player_C|SetCanLayEgg (Variables|Default|GetBp%20player) true)))))
      (:then_1
        (if (Variables|/Game/Blureprints/BP_player.BP_player_C|GetCanLayEgg _bp_player)
          (Game|SpawnActorfromClass "/Game/Character/BP_egg.BP_egg_C" (Math|Transform|MakeTransform (.location (Transformation|GetActorTransform _bp_player)) "0, 0, 0" "1.000000,1.000000,1.000000") "Undefined" "MultiplyWithRoot" 0 0))))))

(event Input|EnhancedActionEvents|EnhancedInputActionIA_Move
  (params (ActionValue :type Vector%202D%20Structure) (ElapsedSeconds :type Float%20%28double-precision%29) (TriggeredSeconds :type Float%20%28double-precision%29) (InputAction :type Input%20Action%20Object%20Reference :default "/Game/Input/Actions/IA_Move.IA_Move"))
  (bind (_x _y) (Math|Vector2D|BreakVector2D ActionValue))
  (:Triggered
    (Pawn|Input|AddMovementInput (Pawn|GetControlledPawn) (Math|Vector|MakeVector _y _x 0.0) 1.0 false))
  (:Completed
    (AI|Navigation|StopMovement)))

(event EventBeginPlay
  (bind _returnvalue (PlayerController|LocalPlayerSubsystems|GetEnhancedInputLocalPlayerSubsystem))
  ;[0.05098 0.05098 0.05098] Add Mapping Context
  (Utilities|IsValid _returnvalue
    (:Is%20Valid
      (Input|AddMappingContext _returnvalue "/Game/Input/IMC_Default.IMC_Default" 0 "(bIgnoreAllPressedKeysUntilRelease=True,bForceImmediately=False,bNotifyUserSettings=False)")
      (Utilities|FlowControl|Sequence
        (:then_0
          (bind _asbp_player (Utilities|Casting|CastToBP_player (Pawn|GetControlledPawn)))
          (Utilities|IsValid _asbp_player
            (:Is%20Valid
              (Variables|Default|SetBp%20player _asbp_player))))
        (:then_1
          (bind _outactors (Actor|GetAllActorsOfClass "/Game/Blureprints/BP_Camera.BP_Camera_C"))
          (bind _output_get (Variables|Default|Setbp%20camera (Utilities|Array|Get(acopy) _outactors)))
          (Game|Player|SetViewTargetwithBlend _output_get 0.0 "VTBlend_Linear" 0.0 false))))))

(fn ConstructionScript)

(fn Moveto
  (params (Location :type Vector))
  (AI|Navigation|SimpleMovetoLocation self Location)
  (Niagara|SpawnSystematLocation (Variables|Input|GetFXCursor) Location))

(fn Follow
  (params (Location :type Vector))
  (bind _returnvalue (Pawn|GetControlledPawn))
  (Pawn|Input|AddMovementInput _returnvalue (Math|Vector|GetUnitDirection(Vector) (Transformation|GetActorLocation _returnvalue) Location) 1.0 false))

(fn GetLocationUnderCursor
  (bind _hitresult (Game|Player|GetHitResultUnderCursorbyChannel "TraceTypeQuery1" true))
  (bind (_bblockinghit _binitialoverlap _time _distance _location) (Collision|BreakHitResult _hitresult))
  (return _bblockinghit _location))

(fn GetLocationUnderFinger
  (bind _hitresult (Class|PlayerController|GetHitResultUnderFingerbyChannel "Touch1" "TraceTypeQuery1" false))
  (bind (_bblockinghit _binitialoverlap _time _distance _location) (Collision|BreakHitResult _hitresult))
  (return _bblockinghit _location))
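; Game mode for a roach colony game, won when more than 50 roaches exist and lost when no egg remains for respawn.
; A throttled Tick counts roaches, keeps food topped up at random positions and respawns a missing player.
; A one-second timer drains a lifespan taken from the game instance; at zero the player becomes food and respawns from an egg.
; End screens pause that timer, but only losing sets the game-end flag.
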(event Custom|LifeCountDown
  (bind _returnvalue (Game|GetPlayerCharacter 0))
  ;[1 1 1] LifeCountDown
  (if (> (Variables|Default|GetLife) 0)
    (Math|Integer|DecrementInt (Variables|Default|GetLife))
    (else
      (Utilities|IsValid _returnvalue
        (:Is%20Valid
          (Game|SpawnActorfromClass "/Game/Blureprints/BP_food.BP_food_C" (Math|Transform|MakeTransform (Transformation|GetActorLocation _returnvalue) "0, 0, 0" "1.000000,1.000000,1.000000") "AdjustIfPossibleButAlwaysSpawn" "MultiplyWithRoot" 0 3 0)
          (Actor|DestroyActor _returnvalue)
          (CallFunction|TrytoRespawnPlayer)
          (Variables|Default|SetLife (Variables|Default|GetMaxLife)))))))

(event Custom|Try%20to%20Respawn%20player
  ;[1 1 1] Try to Respawn Player
  (bind _outactors (Actor|GetAllActorsOfClass "/Game/Blureprints/BP_egg.BP_egg_C"))
  (if (Utilities|Array|IsNotEmpty _outactors)
    (Variables|Default|Setegg (Utilities|Array|Get(acopy) _outactors))
    (CallFunction|RespawnPlayer)
    (else
      (CallFunction|PlayerLose)
      (Variables|Default|SetIsGameEnd true))))

(event Custom|Player%20WIn
  (Utilities|IsValid (Variables|Default|GetWb%20player%20win)
    (:Is%20Valid
      _)
    (:Is%20Not%20Valid
      (bind _returnvalue (UserInterface|CreateWidget "/Game/UI/WB_Win.WB_Win_C"))
      (bind _output_get (Variables|Default|SetWb%20player%20win _returnvalue))))
  (UserInterface|Viewport|AddtoViewport _output_get 0)
  (Utilities|Time|PauseTimerbyHandle (Variables|Default|Gettimer1)))

(event Custom|RespawnPlayer
  (bind _egg (Variables|Default|Getegg))
  (bind _returnvalue (Transformation|GetActorTransform _egg))
  (bind _returnvalue_2 (Game|SpawnActorfromClass "/Game/Blureprints/BP_player.BP_player_C" (Math|Transform|MakeTransform (Math|Vector|MakeVector (.x (.location _returnvalue)) (.y (.location _returnvalue)) 1e+02) "0, 0, 0" "1.000000,1.000000,1.000000") "AdjustIfPossibleButAlwaysSpawn" "MultiplyWithRoot" 0 0))
  (Pawn|Possess (Game|GetPlayerController 0) _returnvalue_2)
  (bind _outactors (Actor|GetAllActorsOfClass "/Game/Blureprints/BP_Camera.BP_Camera_C"))
  (Game|Player|SetViewTargetwithBlend (Game|GetPlayerController 0) (Utilities|Array|Get(acopy) _outactors) 0.0 "VTBlend_Linear" 0.0 false))

(event Custom|Player%20lose
  (Utilities|IsValid (Variables|Default|Getwb%20player%20lose)
    (:Is%20Valid
      _)
    (:Is%20Not%20Valid
      (bind _returnvalue (UserInterface|CreateWidget "/Game/UI/WB_Lose.WB_Lose_C"))
      (bind _output_get (Variables|Default|Setwb%20player%20lose _returnvalue))))
  (UserInterface|Viewport|AddtoViewport _output_get 0)
  (Utilities|Time|PauseTimerbyHandle (Variables|Default|Gettimer1)))

(event Custom|Try%20to%20SpawnFood
  (bind _gamearea_righttopcorner (Variables|Default|GetGameArea_RightTopCorner))
  (bind _outactors (Actor|GetAllActorsOfClass "/Game/Blureprints/BP_food.BP_food_C"))
  (if (< (Utilities|Array|Length _outactors) 2)
    (Game|SpawnActorfromClass "/Game/Blureprints/BP_food.BP_food_C" (Math|Transform|MakeTransform (Math|Vector|MakeVector (Math|Random|RandomFloatinRange 2.3e+02 (.x _gamearea_righttopcorner)) (Math|Random|RandomFloatinRange 2.6e+02 (.y _gamearea_righttopcorner)) 0.0) "0, 0, 0" "1.000000,1.000000,1.000000") "AdjustIfPossibleButAlwaysSpawn" "MultiplyWithRoot" 0 (Math|Random|RandomInteger 2) 0)))

(event EventBeginPlay
  (Utilities|FlowControl|Sequence
    (:then_0
      (Variables|Default|SetMaxLife (Variables|/Game/Blureprints/MyGameInfo.MyGameInfo_C|GetMaxRoact (.AsMy%20Game%20Info (Utilities|Casting|CastToMyGameInfo (Game|GetGameInstance))))))
    (:then_1
      (Variables|Default|SetLife (Variables|Default|GetMaxLife)))
    (:then_2
      (bind _returnvalue (Utilities|Time|SetTimerbyEvent (delegate Custom|LifeCountDown) 1.0 true))
      (Variables|Default|Settimer1 _returnvalue))))

(event EventTick
  (params (DeltaSeconds :type Float%20%28single-precision%29))
  (Utilities|FlowControl|Delay 0.2)
  (if (not (Variables|Default|GetIsGameEnd))
    (Utilities|FlowControl|Sequence
      (:then_0
        (bind _outactors (Actor|GetAllActorsOfClass "/Game/AI/Roach/BP_Roach.BP_Roach_C"))
        (Variables|Default|SetNumber%20of%20Roacts (Utilities|Array|Length _outactors))
        (if (> (Utilities|Array|Length _outactors) 50)
          (CallFunction|PlayerWin)))
      (:then_1
        (CallFunction|TrytoSpawnFood)
        (Utilities|IsValid (Game|GetPlayerCharacter 0)
          (:Is%20Not%20Valid
            (CallFunction|TrytoRespawnPlayer)))))))

(fn ConstructionScript)